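; Game mode for an asteroid game that drives the countdown HUD, score display and game over screen.
; BeginPlay creates the HUD widget and adds it to the viewport.
; CountDownTimerElapsed renews the timer and score if the DestroyAsteroid flag is set, then always notifies the HUD and clears the flag.
; FinishGame shows a game over widget with the final score.
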(event EventBeginPlay
  (bind _returnvalue (UserInterface|CreateWidget "/Game/DEV/UI/WBP_HUD.WBP_HUD_C"))
  (bind _output_get (Variables|Default|SetHUD _returnvalue))
  (UserInterface|Viewport|AddtoViewport _output_get 0))

(event EventTick
  (params (DeltaSeconds :type Float%20%28single-precision%29)))

(event EventCountDownTimerElapsed
  (bind _hud (Variables|Default|GetHUD))
  ;[1 1 1] Interaction with UI
  (if (Variables|Default|GetbDestroyAsteroid)
    (Default|RenewTimer _hud (Variables|Default|GetCount))
    (Default|SetScore _hud (Variables|Default|GetTotalScore)))
  (Default|OnCountDownTimer _hud)
  (Variables|Default|SetbDestroyAsteroid false))

(event EventFinishGame
  (bind _returnvalue (UserInterface|CreateWidget "/Game/DEV/UI/WBP_GameOver.WBP_GameOver_C"))
  (Default|SetFinalScore _returnvalue (Variables|Default|GetTotalScore))
  (UserInterface|Viewport|AddtoViewport _returnvalue 0))

(fn ConstructionScript)