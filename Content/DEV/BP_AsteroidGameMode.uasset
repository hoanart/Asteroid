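; Game mode for an asteroid game that owns the HUD and relays countdown timer updates to it.
; On BeginPlay it creates WBP_HUD and adds it to the viewport.
; CountDownTimerElapsed renews the HUD timer with Count if the DestroyAsteroid flag is set, then always notifies the HUD and clears the flag.
; Nothing in these graphs starts the timer or sets the flag.
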(event EventBeginPlay
  (bind _returnvalue (UserInterface|CreateWidget "/Game/DEV/UI/WBP_HUD.WBP_HUD_C"))
  (bind _output_get (Variables|Default|SetHUD _returnvalue))
  (UserInterface|Viewport|AddtoViewport _output_get 0))

(event EventTick
  (params (DeltaSeconds :type Float%20%28single-precision%29)))

(event EventCountDownTimerElapsed
  (bind _hud (Variables|Default|GetHUD))
  (if (Variables|Default|GetbDestroyAsteroid)
    (Default|RenewTimer _hud (Variables|Default|GetCount)))
  (Default|OnCountDownTimer _hud)
  (Variables|Default|SetbDestroyAsteroid false))

(fn ConstructionScript)